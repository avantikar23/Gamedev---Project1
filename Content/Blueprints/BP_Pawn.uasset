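; BP_Pawn is a pawn Blueprint that equips itself with a BP_GUN1 actor when play begins.
; BeginPlay spawns the gun at the Scene component's transform and attaches its root to that component, snapping location, rotation and scale.
; It also sets the BPGUN and PlayerStart1 variables, and the construction script is empty.
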(event EventBeginPlay
  (bind _scene (Variables|Default|GetScene))
  (bind _returnvalue (Transformation|GetWorldTransform _scene))
  (bind _returnvalue_2 (Game|SpawnActorfromClass "/Game/BP_GUN1.BP_GUN1_C" (Math|Transform|MakeTransform (Math|Transform|TransformLocation _returnvalue "0, 0, 0") (Math|Transform|TransformRotation _returnvalue "0, 0, 0") "1.000000,1.000000,1.000000") "Undefined" "OverrideRootScale" 0 0))
  (Variables|Default|SetBP_GUN "/Game/BP_GUN1.BP_GUN1_C")
  (Transformation|AttachComponentToComponent (Variables|/Script/Engine.Actor|GetRootComponent _returnvalue_2) (Variables|Default|GetScene) "" "SnapToTarget" "SnapToTarget" "SnapToTarget" true)
  (Variables|Default|SetPlayerStart1 "/Script/Engine.PlayerStart"))

(fn ConstructionScript)